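; BP_Enemy is an armed AI enemy character that patrols between two points.
; On BeginPlay it spawns a BP_AR, attaches it to a holster socket and writes the current patrol point to the Blackboard.
; Overlapping either patrol point swaps the target and updates that key.
; Equip and holster events play montages that toggle CombatReady on completion, while functions report the weapon slot and a camera-traced look-at point.
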(event Custom|HolsterAIWeapon
  (if (Variables|Default|GetCombatReady)
    (Animation|Montage|PlayMontage (Variables|Character|GetMesh) "/Game/LQProject/Assets/Character/Animations/AM_HolsterWeapon_BR.AM_HolsterWeapon_BR"
      (:OnCompleted
        (Variables|Default|SetCombatReady false)))))

(event Custom|EquipAIWeapon
  (if (not (Variables|Default|GetCombatReady))
    (Animation|Montage|PlayMontage (Variables|Character|GetMesh) "/Game/LQProject/Assets/Character/Animations/AM_EquipWeapon_BR.AM_EquipWeapon_BR"
      (:OnCompleted
        (Variables|Default|SetCombatReady true)
        (Development|PrintString "CombatReady")))))

(event EventBeginPlay
  ;[1 1 1] 绑定武器
  (bind _returnvalue (Game|SpawnActorfromClass "/Game/BluePrints/Weapons/AR/BP_AR.BP_AR_C" (Transformation|GetActorTransform) "Undefined" 0 0))
  (bind _output_get (Variables|Default|SetWeapon _returnvalue))
  (Default|GetWeapon _output_get self)
  (Transformation|AttachComponentToComponent (Variables|Default|GetWeapon) (Variables|Character|GetMesh) "HolsterBRSocket" "SnapToTarget" "SnapToTarget" "SnapToTarget" true)
  (AI|Components|Blackboard|SetValueasObject (AI|GetBlackboard self) (Utilities|Name|MakeLiteralName "PatrolPoint") (Variables|Default|GetCurrentPatrolPoint)))

(event EventTick
  (params (DeltaSeconds :type Float%20%28single-precision%29))
  (|CallParentFunction 0.0))

(event Game|Damage|EventAnyDamage
  (params (Damage :type Float%20%28single-precision%29) (DamageType :type Damage%20Type%20Object%20Reference) (InstigatedBy :type Controller%20Object%20Reference) (DamageCauser :type Actor%20Object%20Reference)))

(event Collision|EventActorBeginOverlap
  (params (OtherActor :type Actor%20Object%20Reference))
  ;[1 1 1] 更新巡逻点
  (if (== OtherActor (Variables|Default|GetPatrolPoint1))
    (Variables|Default|SetCurrentPatrolPoint (Variables|Default|GetPatrolPoint2))
    (AI|Components|Blackboard|SetValueasObject (AI|GetBlackboard self) (Utilities|Name|MakeLiteralName "PatrolPoint") (Variables|Default|GetCurrentPatrolPoint) :!label _label)
    (elif (== OtherActor (Variables|Default|GetPatrolPoint2))
      (Variables|Default|SetCurrentPatrolPoint (Variables|Default|GetPatrolPoint1))
      (goto _label))))

(fn ConstructionScript
  (|CallParentFunction))

(fn PickUpScanner
  (return "" false))

(fn GetCurrentWeaponSlot
  (return (Variables|Default|GetWeapon) "NewEnumerator0" "HolsterBRSocket"))

(fn ActorLookatDirection
  (bind (_outhit _returnvalue) (Collision|LineTraceByChannel (Transformation|GetWorldLocation (Variables|Default|GetFollowCamera)) (* (Math|Vector|GetForwardVector (Pawn|GetControlRotation :!class /Script/Engine.Pawn)) 1e+04) "TraceTypeQuery1" false 0 "ForOneFrame"))
  (return (Math|Vector|SelectVector (.Location (Collision|BreakHitResult _outhit)) (.TraceEnd (Collision|BreakHitResult _outhit)) _returnvalue)))