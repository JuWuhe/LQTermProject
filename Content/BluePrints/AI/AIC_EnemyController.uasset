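; Enemy AI controller that runs the default enemy behavior tree and tracks the player through AI Perception.
; Sensing an actor tagged Player sets the FindPlayer and PlayerActor blackboard keys and cancels any pending lost-target timer.
; Losing it clears FindPlayer immediately, while PlayerActor is cleared only after a five-second delay.
; Tick copies the stored player character's Alive state into the PlayerActorAlive key.
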(event OnTargetPerceptionUpdated(AIPerception)
  (params (Actor :type Actor%20Object%20Reference) (Stimulus :type AI%20Stimulus%20Structure))
  (Variables|Default|SetActor Actor)
  (if (Actor|ActorHasTag Actor "Player")
    (if (.bSuccessfullySensed (Utilities|Struct|BreakAIStimulus Stimulus))
      (Utilities|Time|ClearandInvalidateTimerbyHandle (Variables|Default|GetLostTargetTime))
      (CallFunction|UpdateFindPlayer true)
      (CallFunction|UpdatePlayerActor (Variables|Default|GetActor))
      (else
        (bind _returnvalue (Utilities|Time|SetTimerbyEvent (delegate Custom|LostTarget) 5.0))
        (Variables|Default|SetLostTargetTime _returnvalue)
        (CallFunction|UpdateFindPlayer false)))))

(event Custom|LostTarget
  (CallFunction|UpdatePlayerActor))

(event EventBeginPlay
  ;[1 1 1] 运行行为树
  (AI|RunBehaviorTree "/Game/BluePrints/AI/BT_DefaultEnemy.BT_DefaultEnemy"))

(event EventTick
  (params (DeltaSeconds :type Float%20%28single-precision%29))
  (bind _self self)
  (bind _blackboard (Variables|Default|GetBlackboard _self))
  (Utilities|FlowControl|Sequence
    (:then_0
      (bind _asbp_base_character (Utilities|Casting|CastToBP_BaseCharacter (AI|Components|Blackboard|GetValueasObject _blackboard (Utilities|Name|MakeLiteralName "PlayerActor"))))
      (AI|Components|Blackboard|SetValueasBool _blackboard (Utilities|Name|MakeLiteralName "PlayerActorAlive") (Variables|/Game/BluePrints/BP_BaseCharacter.BP_BaseCharacter_C|GetAlive _asbp_base_character)))))

(fn ConstructionScript)

(fn UpdateFindPlayer
  (params (FindPlayer :type Boolean))
  (AI|Components|Blackboard|SetValueasBool (Variables|Default|GetBlackboard) (Utilities|Name|MakeLiteralName "FindPlayer") FindPlayer)
  (return))

(fn UpdatePlayerActor
  (params (Actor :type Actor%20Object%20Reference))
  (AI|Components|Blackboard|SetValueasObject (Variables|Default|GetBlackboard) (Utilities|Name|MakeLiteralName "PlayerActor") Actor)
  (return))