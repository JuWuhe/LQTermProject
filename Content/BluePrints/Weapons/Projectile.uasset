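; Projectile actor for weapons that bounces off surfaces, pushes what it overlaps and removes itself.
; On each bounce, it scales velocity by a factor looked up from the hit physical material in the SpeedDown map, with a default fallback.
; On overlap, it applies an impulse to both components along its negated world location, not its travel direction, then destroys itself.
; Tick destroys it shortly after its velocity reaches zero.
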(event OnComponentBeginOverlap(CollisionComponent)
  (params (OverlappedComponent :type Primitive%20Component%20Object%20Reference) (OtherActor :type Actor%20Object%20Reference) (OtherComp :type Primitive%20Component%20Object%20Reference) (OtherBodyIndex :type Integer) (bFromSweep :type Boolean) (SweepResult :type Hit%20Result%20Structure%20%28by%20ref%29))
  (Physics|AddImpulse OtherComp (* (* (Transformation|GetActorLocation) -1.0) 1e+03) "None" false)
  (Actor|DestroyActor))

(event OnProjectileBounce(Projectile)
  (params (ImpactResult :type Hit%20Result%20Structure%20%28by%20ref%29) (ImpactVelocity :type Vector%20%28by%20ref%29 :default "0, 0, 0"))
  (bind _physmat (Collision|BreakHitResult ImpactResult))
  (bind _projectile (Variables|MyProjectile|GetProjectile))
  (bind _speeddown (Variables|Default|GetSpeedDown))
  (bind (_value _returnvalue) (Utilities|Map|Find _speeddown _physmat))
  (if _returnvalue
    (Variables|Default|SetSpeedDownFloat _value)
    (else
      (Variables|Default|SetSpeedDownFloat 0.6)))
  (Variables|/Script/Engine.MovementComponent|SetVelocity _projectile (* (Variables|/Script/Engine.MovementComponent|GetVelocity _projectile) (Variables|Default|GetSpeedDownFloat))))

(event EventTick
  (params (DeltaSeconds :type Float%20%28single-precision%29))
  (if (Math|Vector|Equal(Vector) (Transformation|GetVelocity) "0,0.000000,0.000000" 0.0001)
    (Utilities|FlowControl|Delay 0.2)
    (Actor|DestroyActor)))

(fn ConstructionScript)