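; Base weapon actor that a character picks up, fires and reloads, and that reports its type for a weapon panel.
; On pickup it stores the owner, disables physics and collision, and derives an aim baseline offset from the sight socket for right-hand IK.
; Semi-auto fire is gated by chambered rounds and DoOnce; a montage notify spawns a projectile aimed at the owner's look point, or along the muzzle when looking behind.
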(event Custom|MagReloadWeapon
  ;[1 1 1] 换弹动画
  (Animation|Montage|PlayMontage (Variables|Default|GetSkeletalMesh) "/Game/LQProject/Assets/Weapon/Animations/AM_AR_Reload_NoCharge.AM_AR_Reload_NoCharge"))

(event Custom|Fire
  (bind _skeletalmesh (Variables|Default|GetSkeletalMesh))
  (bind _returnvalue (Transformation|GetSocketTransform _skeletalmesh "Muzzle" "RTS_World"))
  ;[1 1 1] 开火
  (switch Utilities|FlowControl|Switch|SwitchonE_FireMode (Variables|Default|GetFireMode)
    (:NewEnumerator1
      ;;[1 1 1] 开火动画
      (Utilities|FlowControl|DoOnce false :!label _label
        (:Completed
          (Animation|Montage|PlayMontage (Variables|/Script/Engine.Character|GetMesh (Variables|Default|GetOwning%20Character)) "/Game/LQProject/Assets/Character/Animations/AM_2HW_ADS_Fire.AM_2HW_ADS_Fire"
            (:then
              (Animation|Montage|PlayMontage (Variables|Default|GetSkeletalMesh) "/Game/LQProject/Assets/Weapon/Animations/AM_AR_Fire.AM_AR_Fire"
                (:OnBlendOut
                  (goto _label Reset))
                (:OnNotifyBegin
                  ;;[1 1 1] 生成子弹
                  (bind _returnvalue_2 (Game|SpawnActorfromClass "/Game/BluePrints/Weapons/BP_BaseProjectile.BP_BaseProjectile_C" (Math|Transform|MakeTransform (.location _returnvalue) (.rotation _returnvalue) "1,1,1") "Undefined" self (Variables|Default|GetOwning%20Character)))
                  (Utilities|IsValid _returnvalue_2
                    (:Is%20Valid
                      (Variables|/Game/BluePrints/Weapons/BP_BaseProjectile.BP_BaseProjectile_C|SetOwningWeapon _returnvalue_2 self)
                      (Variables|/Script/Engine.MovementComponent|SetVelocity (Variables|/Game/BluePrints/Weapons/BP_BaseProjectile.BP_BaseProjectile_C|GetProjectileMovement _returnvalue_2) (* (select (> (Math|Float|Absolute(Float) (Variables|/Game/BluePrints/BP_BaseCharacter.BP_BaseCharacter_C|GetYaw (Variables|Default|GetOwning%20Character))) 9e+01) (Math|Vector|GetForwardVector (Transformation|GetSocketRotation (Variables|Default|GetSkeletalMesh) "Muzzle")) (Math|Vector|Normalize (- (Variables|/Game/BluePrints/BP_BaseCharacter.BP_BaseCharacter_C|GetLookAtPoint (Variables|Default|GetOwning%20Character)) (Transformation|GetSocketLocation (Variables|Default|GetSkeletalMesh) "Muzzle")))) (Variables|Default|GetMuzzleVelocity))))))))))))))

(event EventFirePressed
  ;[1 1 1] 开火
  (if (> (Variables|Default|GetRoundsInChamber) 0)
    (CallFunction|Fire)))

(event EventGetWeapon
  (params (OwningCharacter :type BP%20Base%20Character%20Object%20Reference))
  (Variables|Default|SetOwning%20Character OwningCharacter)
  ;[1 1 1] 设置物理
  (Physics|SetSimulatePhysics (Variables|Default|GetSkeletalMesh) false)
  (Collision|SetActorEnableCollision false)
  (Variables|Default|SetAimBaselineOffset (- (Class|KismetAnimationLibrary|DistanceBetweenTwoSocketsandMapRange (Variables|Default|GetSkeletalMesh) "Root" "RTS_World" "Sight" "RTS_World" false 0.0 0.0 0.0 0.0) 13.5)) ; Use in BPI_Character to RightHandIK
)

(fn ConstructionScript)

(fn GetWeaponPanelInfo
  (return (Utilities|Struct|MakeWeaponPanelInfo self (Variables|Default|GetWeaponType))))