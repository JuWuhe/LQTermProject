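; TPS game mode that sets up player logins, handles respawning and starts the match's RemainingTime at 600 on the game state.
; On login, the server sorts PlayerStarts into Player1 and Player2 pools by tag, numbers the player by player count and calls ClientPostLogin on the controller.
; RespawnPlayer destroys the current pawn, then spawns and possesses a BP_BaseCharacter at one of two random starts, using Player1's pool for the first PlayerArray entry and Player2's otherwise.
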(event Custom|RespawnPlayer
  (params (PlayerController :type My%20Player%20Controller%20Object%20Reference))
  (bind _returnvalue (Pawn|GetControlledPawn PlayerController))
  (bind _returnvalue_2 (Math|Random|RandomIntegerinRange 0 1))
  (Utilities|IsValid _returnvalue
    (:Is%20Valid
      (Actor|DestroyActor _returnvalue))
    (:Is%20Not%20Valid
      _))
  (if (== (Variables|/Script/Engine.PlayerState|GetPlayerId (Variables|/Script/Engine.Controller|GetPlayerState PlayerController)) (Variables|/Script/Engine.PlayerState|GetPlayerId (Utilities|Array|Get(acopy) (Variables|/Script/Engine.GameStateBase|GetPlayerArray (Game|GetGameState)))))
    (bind _returnvalue_3 (Game|SpawnActorfromClass "/Game/BluePrints/BP_BaseCharacter.BP_BaseCharacter_C" (Transformation|GetActorTransform (Utilities|Array|Get(acopy) (Variables|Default|GetPlayer1) _returnvalue_2)) "Undefined" 0 0))
    (Pawn|Possess PlayerController _returnvalue_3)
    (else
      (bind _returnvalue_4 (Game|SpawnActorfromClass "/Game/BluePrints/BP_BaseCharacter.BP_BaseCharacter_C" (Transformation|GetActorTransform (Utilities|Array|Get(acopy) (Variables|Default|GetPlayer2) _returnvalue_2)) "Undefined" 0 0))
      (Pawn|Possess PlayerController _returnvalue_4))))

(event EventBeginPlay
  (bind _asmy_game_state (Utilities|Casting|CastToMyGameState (Game|GetGameState)))
  (Variables|/Game/BluePrints/Game/MyGameState.MyGameState_C|SetRemainingTime _asmy_game_state 600))

(event EventPostLogin
  (params (NewPlayer :type Player%20Controller%20Object%20Reference))
  ;[1 1 1] PostLogin
  (Networking|SwitchHasAuthority
    (:Authority
      (bind _outactors (Actor|GetAllActorsOfClass "/Script/Engine.PlayerStart"))
      (for _array_element _outactors
        (if (Utilities|Name|Equal(Name) (Variables|/Script/Engine.PlayerStart|GetPlayerStartTag _array_element) "Player1")
          (Utilities|Array|AddUnique (Variables|Default|GetPlayer1) _array_element)
          (else
            (Utilities|Array|AddUnique (Variables|Default|GetPlayer2) _array_element))))
      (bind _asmy_player_state (Utilities|Casting|CastToMyPlayerState (Variables|/Script/Engine.Controller|GetPlayerState NewPlayer)))
      (Variables|/Game/BluePrints/Game/MyPlayerState.MyPlayerState_C|SetPlayerNumber _asmy_player_state (Utilities|Array|Length (Variables|/Script/Engine.GameStateBase|GetPlayerArray (Game|GetGameState))))
      (bind _asmy_player_controller (Utilities|Casting|CastToMyPlayerController NewPlayer))
      (Default|ClientPostLogin _asmy_player_controller))))

(fn ConstructionScript)