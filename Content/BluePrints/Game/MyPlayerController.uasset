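; Player controller that owns the game's main HUD and ranking board widgets and switches between them.
; On begin play it shows the mouse cursor; ShowUIWidget creates both widgets for the local controller and displays only the HUD.
; Showing the ranking loads its data, makes the HUD non-interactive, sets UI-only input and clears the touch interface; hiding it restores game input and touch controls.
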(event EventBeginPlay
  (Variables|Default|SetbShowMouseCursor true))

(fn ConstructionScript)

(fn ShowUIWidget
  (if (Pawn|IsLocalPlayerController)
    (bind _returnvalue (UserInterface|CreateWidget "/Game/BluePrints/Widgets/MyHud.MyHUD_C" self))
    (Variables|Default|SetMainMenu _returnvalue)
    (UserInterface|Viewport|AddtoViewport _returnvalue 0)
    (bind _returnvalue_2 (UserInterface|CreateWidget "/Game/BluePrints/Widgets/RankingBoard.RankingBoard_C" self))
    (Variables|Default|SetRankingMenu _returnvalue_2)))

(fn HideRankWidget
  (Widget|RemovefromParent (Variables|Default|GetRankingMenu))
  (Input|SetInputModeGameOnly self)
  (Class|PlayerController|ActivateTouchInterface self (Variables|Default|GetTouchInterface))
  (Widget|SetVisibility (Variables|Default|GetMainMenu) "SelfHitTestInvisible"))

(fn ShowRankWidget
  (UserInterface|Viewport|AddtoViewport (Variables|Default|GetRankingMenu) 0)
  (Widget|SetVisibility (Variables|Default|GetMainMenu) "HitTestInvisible")
  (Default|LoadData (Variables|Default|GetRankingMenu))
  (Input|SetInputModeUIOnly self (Variables|Default|GetRankingMenu) "DoNotLock")
  (Class|PlayerController|ActivateTouchInterface self))